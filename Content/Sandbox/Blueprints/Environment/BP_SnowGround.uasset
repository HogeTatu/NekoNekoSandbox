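; Snow ground actor that records the player's trail in a runtime height map texture and gradually covers it over again.
; Each tick it raises a CPU byte array toward white, then darkens texels near player 0 by a distance-based curve, keeping the minimum value.
; The array is re-uploaded to a texture bound to the mesh's dynamic material.
; Player position maps to texels assuming the floor is centered on the world origin.
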(event EventBeginPlay
  (bind _returnvalue (Rendering|Material|CreateDynamicMaterialInstance (Variables|Default|GetStaticMesh) 0 0 :!class /Script/Engine.PrimitiveComponent))
  (Variables|Default|SetDynamicMaterialInstance _returnvalue)
  (CallFunction|UpdateTexture)
  (Rendering|Material|SetTextureParameterValue (Variables|Default|GetDynamicMaterialInstance) "Texture" (Class|TextureBuildComponent|GetTexture (Variables|Default|GetTextureBuild))))

(event EventTick
  (params (DeltaSeconds :type Float%20%28single-precision%29))
  (CallFunction|UpdateHeightMap DeltaSeconds)
  (CallFunction|UpdateTexture))

(fn ConstructionScript
  (Utilities|Array|Resize (Variables|Default|GetTextureData) (* (Variables|Default|GetTextureWidth) (Variables|Default|GetTextureHeight) 4))
  (Class|ArrayFunctionLibrary|AddByteValuetoArraywithClamp (Variables|Default|GetTextureData) 255 0 255))

(fn UpdateTexture
  (Class|TextureBuildComponent|UpdateTexture (Variables|Default|GetTextureBuild) (Variables|Default|GetTextureData) (Variables|Default|GetTextureWidth) (Variables|Default|GetTextureHeight) "PF_R8G8B8A8") ; テクスチャ更新
)

(fn UpdateHeightMap
  (params (DeltaSeconds :type Float%20%28single-precision%29))
  (bind _floorsize (Variables|Default|GetFloorSize))
  (LocalVariables|SetDeltaSeconds_ DeltaSeconds)
  (Utilities|FlowControl|Sequence
    (:then_0
      (Class|ArrayFunctionLibrary|AddByteValuetoArraywithClamp (Variables|Default|GetTextureData) (Math|Conversions|ToByte(Integer) (Math|Float|Round (* (Variables|Default|GetSnowCoverSpeed) (LocalVariables|GetDeltaSeconds_)))) 0 255))
    (:then_1
      (bind _output_get (LocalVariables|SetPlayerLocation (Transformation|GetActorLocation (Game|Player|GetPlayerPawn 0))))
      (LocalVariables|SetBaseX (Math|Float|Floor (* (Variables|Default|GetTextureWidth) (- (/ (.y _output_get) (.x _floorsize)) -0.5))))
      (LocalVariables|SetBaseY (Math|Float|Floor (* (Variables|Default|GetTextureHeight) (- (/ (.x _output_get) (.y _floorsize)) -0.5))))
      (for _index (range (Math|Integer|Max(Integer) (- (LocalVariables|GetBaseY) 10)) (Math|Integer|Min(Integer) (+ (LocalVariables|GetBaseY) 10) (Variables|Default|GetTextureHeight)))
        (LocalVariables|SetY _index)
        (for _index_2 (range (Math|Integer|Max(Integer) (- (LocalVariables|GetBaseX) 10)) (Math|Integer|Min(Integer) (+ (LocalVariables|GetBaseX) 10) (Variables|Default|GetTextureWidth)))
          (LocalVariables|SetX _index_2)
          (LocalVariables|SetData (Math|Conversions|ToByte(Integer) (Math|Integer|Clamp(Integer) (Math|Float|Round (* (- 1.0 (Math|Curves|GetFloatValue (LocalVariables|GetOffsetCurve) (Math|Float|Sqrt (Math|Conversions|ToFloat(Integer) (+ (* (- (LocalVariables|GetX) (LocalVariables|GetBaseX)) (- (LocalVariables|GetX) (LocalVariables|GetBaseX))) (* (- (LocalVariables|GetY) (LocalVariables|GetBaseY)) (- (LocalVariables|GetY) (LocalVariables|GetBaseY)))))))) 256.0)) 0 255)))
          (for _index_3 (range 0 2)
            (Utilities|Array|SetArrayElem (Variables|Default|GetTextureData) (+ _index_3 (* (+ (LocalVariables|GetX) (* (LocalVariables|GetY) (Variables|Default|GetTextureWidth))) 4)) (Class|KismetMathLibrary|BMin (Utilities|Array|Get(acopy) (Variables|Default|GetTextureData) (+ _index_3 (* (+ (LocalVariables|GetX) (* (LocalVariables|GetY) (Variables|Default|GetTextureWidth))) 4))) (LocalVariables|GetData)))))))))