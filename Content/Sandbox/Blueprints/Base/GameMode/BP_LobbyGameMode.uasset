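; BP_LobbyGameMode is the lobby game mode, which manages a shared loading screen overlay.
; It creates a UI_Loading widget on BeginPlay and keeps it for reuse.
; PushLoading and PopLoading reference-count requests through LoadCount, adding the widget at a high Z-order when the count reaches one and removing it when the count returns to zero.
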(event EventPushLoading
  (bind _result (Math|Integer|IncrementInt (Variables|Loading|GetLoadCount))
    (:%20%20
      (if (== _result 1)
        (UserInterface|Viewport|AddtoViewport (Variables|Loading|GetLoadingWidget) 1000)))))

(event EventBeginPlay
  (bind _returnvalue (UserInterface|CreateWidget "/Game/Sandbox/UI/UI_Loading.UI_Loading_C"))
  (Variables|Loading|SetLoadingWidget _returnvalue))

(event EventPopLoading
  (bind _result (Math|Integer|DecrementInt (Variables|Loading|GetLoadCount))
    (:%20%20
      (if (== _result 0)
        (Widget|RemovefromParent (Variables|Loading|GetLoadingWidget))))))

(fn ConstructionScript)