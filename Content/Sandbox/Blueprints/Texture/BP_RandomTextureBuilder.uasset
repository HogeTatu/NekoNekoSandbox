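; Sandbox actor that progressively fills a texture with random opaque RGBA pixels and shows it on a Billboard.
; The construction script sizes the byte array to width × height × 4.
; Each Tick, while pixels remain, it writes a fixed batch using a running index, then TextureBuild uploads the whole array as R8G8B8A8.
; A DoOnce assigns the built texture as the Billboard sprite after the first upload.
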(event EventTick
  (params (DeltaSeconds :type Float%20%28single-precision%29))
  (Utilities|IsEnabledUpdate
    (:True
      (for _index (range 0 (- (Variables|Default|GetOneFrameUpdatePixel) 1))
        (Utilities|IsEnabledUpdate
          (:True
            (for _index_2 (range 0 2)
              (Utilities|Array|SetArrayElem (Variables|Default|GetTextureData) (+ _index_2 (* (Variables|Default|GetIndex) 4)) (Math|Conversions|ToByte(Integer) (Math|Random|RandomIntegerinRange 0 255))) ; ランダムにテクスチャデータ設定
            )
            (Utilities|Array|SetArrayElem (Variables|Default|GetTextureData) (+ 3 (* (Variables|Default|GetIndex) 4)) 255)
            (Math|Integer|IncrementInt (Variables|Default|GetIndex)))))
      (Class|TextureBuildComponent|UpdateTexture (Variables|Default|GetTextureBuild) (Variables|Default|GetTextureData) (Variables|Default|GetTextureWidth) (Variables|Default|GetTextureHeight) "PF_R8G8B8A8") ; テクスチャ更新
      (Utilities|FlowControl|DoOnce false
        (:Completed
          (Rendering|Components|Sprite|SetSprite (Variables|Default|GetBillboard) (Class|TextureBuildComponent|GetTexture (Variables|Default|GetTextureBuild))) ; テクスチャをビルボードに設定
        )))))

(fn ConstructionScript
  (Utilities|Array|Resize (Variables|Default|GetTextureData) (* (Variables|Default|GetTextureWidth) (Variables|Default|GetTextureHeight) 4)))