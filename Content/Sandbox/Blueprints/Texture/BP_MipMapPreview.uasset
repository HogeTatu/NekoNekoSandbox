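; BP_MipMapPreview is a preview tool that shows mip levels on tagged actors by overriding their materials.
; Its construction script feeds each MipTextures entry into TextureBuild as the mip matching its index, building one 512x512 texture.
; That texture drives a dynamic preview material instance.
; Each run restores previously saved materials, then, if EnablePreview is set, saves and replaces those on primitives of actors matching ReplaceTag.
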(event Custom|UpdateRenderTarget
  (Utilities|FlowControl|Sequence
    (:then_0
      (for (_array_element _array_index) (Variables|Material|GetMipTextures)
        (bind (_data _format _returnvalue) (Class|TextureFunctionLibrary|GetTextureData _array_element))
        (if _returnvalue
          (Class|TextureBuildComponent|UpdateTexture (Variables|Default|GetTextureBuild) _data 512 512 _format _array_index))))
    (:then_1
      (bind _returnvalue_2 (Rendering|Material|CreateDynamicMaterialInstance (Variables|Material|GetMipMapPreviewMaterial) :!class /Script/Engine.KismetMaterialLibrary))
      (Variables|Material|SetMipMapPreviewMaterialInstance _returnvalue_2)
      (Rendering|Material|SetTextureParameterValue (Variables|Material|GetMipMapPreviewMaterialInstance) "Texture" (Class|TextureBuildComponent|GetTexture (Variables|Default|GetTextureBuild))))
    (:then_2
      (CallFunction|RestoreReplacedMaterials)
      (if (Variables|Material|GetEnablePreview)
        (CallFunction|ReplaceMaterials)))))

(fn ConstructionScript
  (CallFunction|UpdateRenderTarget))

(fn RestoreReplacedMaterials
  (for _array_element (Variables|Material|GetReplaceInfoList)
    (for (_array_element_2 _array_index) (.materials _array_element)
      (Rendering|Material|SetMaterial (.primitive _array_element) _array_index _array_element_2)))
  (Utilities|Array|Clear (Variables|Material|GetReplaceInfoList)))

(fn ReplaceMaterials
  (bind _outactors (Actor|GetAllActorswithTag (Variables|Material|GetReplaceTag)))
  (for _array_element _outactors
    (LocalVariables|SetPrimitives (Actor|GetComponentsByClass _array_element "/Script/Engine.PrimitiveComponent"))
    (bind _asprimitive_component (Utilities|Casting|CastToPrimitiveComponent (VehicleSound|GetRootComponent _array_element))
      (:then
        (Utilities|Array|Add (LocalVariables|GetPrimitives) _asprimitive_component))
      (:CastFailed
        _))
    (Utilities|FlowControl|Sequence
      (:then_0
        (for _array_element_2 (LocalVariables|GetPrimitives)
          (Utilities|Array|Clear (LocalVariables|GetMaterials))
          (for _index (range 0 (- (Rendering|Material|GetNumMaterials _array_element_2) 1))
            (Utilities|Array|Add (LocalVariables|GetMaterials) (Rendering|Material|GetMaterial _array_element_2 _index)))
          (if (> (Utilities|Array|Length (LocalVariables|GetMaterials)) 0)
            (Utilities|Array|Add (Variables|Material|GetReplaceInfoList) (Utilities|Struct|MakeST_MipMapPreviewReplaceInfo _array_element_2 (LocalVariables|GetMaterials))))))
      (:then_1
        (for _array_element_3 (LocalVariables|GetPrimitives)
          (for _index_2 (range 0 (- (Rendering|Material|GetNumMaterials _array_element_3) 1))
            (Rendering|Material|SetMaterial _array_element_3 _index_2 (Variables|Material|GetMipMapPreviewMaterialInstance))))))))