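; BP_Notify is a short-lived actor that sends a notify message to actors reached by an expanding radius around it.
; On BeginPlay it creates a dynamic decal material centered on its location and plays a timeline driving circle radius and opacity.
; The same radius resizes a Sphere collision, so each actor that begins overlapping receives OnReceivedNotifyMessage in step with the visual.
; The actor destroys itself when the timeline finishes.
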(event OnComponentBeginOverlap(Sphere)
  (params (OverlappedComponent :type Primitive%20Component%20Object%20Reference) (OtherActor :type Actor%20Object%20Reference) (OtherComp :type Primitive%20Component%20Object%20Reference) (OtherBodyIndex :type Integer) (bFromSweep :type Boolean) (SweepResult :type Hit%20Result%20Structure%20%28by%20ref%29))
  (Class|BPINotifyReceiver|OnReceivedNotify(Message) OtherActor))

(event EventBeginPlay
  (bind _returnvalue (Rendering|Material|CreateDynamicMaterialInstance (Variables|Default|GetDecal) :!class /Script/Engine.DecalComponent))
  (Rendering|Material|SetVectorParameterValue _returnvalue "ActorPosition" (Math|Conversions|ToLinearColor(Vector) (Transformation|GetActorLocation)) :!class /Script/Engine.MaterialInstanceDynamic)
  (bind (_direction _radius _opacity) (Timeline|NotifyTL Play)
    (:Update
      (Rendering|Material|SetScalarParameterValue _returnvalue "CircleRadius" _radius :!class /Script/Engine.MaterialInstanceDynamic)
      (Rendering|Material|SetScalarParameterValue _returnvalue "Opacity" _opacity :!class /Script/Engine.MaterialInstanceDynamic)
      (Components|Sphere|SetSphereRadius (Variables|Default|GetSphere) _radius true))
    (:Finished
      (Actor|DestroyActor))))

(fn ConstructionScript)