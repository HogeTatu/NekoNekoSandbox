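; Web API Blueprint for the Docomo dialogue service that sends an utterance and captures the reply.
; The request filter writes Utt, a hard-coded Japanese user profile and any non-empty Context into the JSON body.
; The response filter reads the reply text and context from the JSON into ResponseUtt and ResponseContext.
; Requests or responses that fail the JSON cast, and responses without a valid accessor, pass through unchanged.
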(fn ExecuteRequestFilter
  (params (Request :type Web%20Api%20Request%20Body%20Object%20Reference))
  (bind _asweb_api_request_body_json (Utilities|Casting|CastToWebApiRequestBodyJson Request)
    (:then
      (LocalVariables|SetRequestBodyJson _asweb_api_request_body_json)
      (Utilities|FlowControl|Sequence
        (:then_0
          (Class|WebApiRequestBodyUrlParam|SetRequestParam (LocalVariables|GetRequestBodyJson) "utt" (Variables|Talk|GetUtt))
          (Class|WebApiRequestBodyUrlParam|SetRequestParam (LocalVariables|GetRequestBodyJson) "nickname" "ほげたつ")
          (Class|WebApiRequestBodyUrlParam|SetRequestParam (LocalVariables|GetRequestBodyJson) "nickname_y" "ホゲタツ")
          (Class|WebApiRequestBodyUrlParam|SetRequestParam (LocalVariables|GetRequestBodyJson) "sex" "男")
          (Class|WebApiRequestBodyUrlParam|SetRequestParam (LocalVariables|GetRequestBodyJson) "bloodtype" "B")
          (Class|WebApiRequestBodyUrlParam|SetRequestParam (LocalVariables|GetRequestBodyJson) "birthdateY" "1988")
          (Class|WebApiRequestBodyUrlParam|SetRequestParam (LocalVariables|GetRequestBodyJson) "birthdateM" "8")
          (Class|WebApiRequestBodyUrlParam|SetRequestParam (LocalVariables|GetRequestBodyJson) "birthdateD" "29")
          (Class|WebApiRequestBodyUrlParam|SetRequestParam (LocalVariables|GetRequestBodyJson) "age" "28")
          (Class|WebApiRequestBodyUrlParam|SetRequestParam (LocalVariables|GetRequestBodyJson) "constellations" "乙女座")
          (Class|WebApiRequestBodyUrlParam|SetRequestParam (LocalVariables|GetRequestBodyJson) "place" "東京"))
        (:then_1
          (if (> (Utilities|String|Len (Variables|Talk|GetContext)) 0)
            (Class|WebApiRequestBodyUrlParam|SetRequestParam (LocalVariables|GetRequestBodyJson) "context" (Variables|Talk|GetContext))))
        (:then_2
          (return (LocalVariables|GetRequestBodyJson)))))
    (:CastFailed
      (return Request))))

(fn ExecuteResponseFilter
  (params (Response :type Web%20Api%20Response%20Body%20Object%20Reference))
  (bind _asweb_api_response_body_json (Utilities|Casting|CastToWebApiResponseBodyJson Response)
    (:then
      (bind (_jsonaccessor _success) (Class|WebApiResponseBodyJson|GetJsonAccessor _asweb_api_response_body_json))
      (if _success
        (Utilities|FlowControl|Sequence
          (:then_0
            (bind (_out _returnvalue) (Class|JsonFunctionLibrary|TryGetStringField _jsonaccessor "utt"))
            (if _returnvalue
              (Variables|Talk|SetResponseUtt _out)))
          (:then_1
            (bind (_out_2 _returnvalue_2) (Class|JsonFunctionLibrary|TryGetStringField _jsonaccessor "context"))
            (if _returnvalue_2
              (Variables|Talk|SetResponseContext _out_2)))
          (:then_2
            (return _asweb_api_response_body_json)))
        (else
          (return Response))))
    (:CastFailed
      (return Response))))